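; Game instance that holds the player's resource stockpile in a map keyed by resource type.
; InitializeResourceMap fills the map from a data table with each resource's name, icon and starting count.
; AddResource and SpendResource write updated structs back, fire change dispatchers and return success, failing on unknown types or, when spending, insufficient count.
; A helper returns the first player's BC_PlayerState_Master.
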(fn `AddResource`
  (params (ResourceType :type "/Game/Blueprints/Enums/E_ResourceTypes Enum (by ref)") (Count :type Integer))
  (returns (`Success?` :type Boolean))
  (bind (_value _returnvalue) (`BlueprintMapLibrary.Map_Find` (`self.ResourcesMap`) ResourceType))
  (if _returnvalue
    (bind _structout (setmembers `/Game/Blueprints/Structs/S_ResourceStorage` :`StructRef` _value :`Count` (+ (`.Count_8_443DEF174797DB10D7CFFD9D13AF4340` (break `/Game/Blueprints/Structs/S_ResourceStorage` _value)) Count)))
    (`BlueprintMapLibrary.Map_Add` (`self.ResourcesMap`) ResourceType _structout)
    (`self.OnResourceAdded` ResourceType _structout)
    (return true)
    (else
      (return false))))

(fn `Get Player State`
  (returns (`Player State` :type "/Game/Blueprints/Player/BC_PlayerState_Master Object Reference"))
  (bind _asbc_player_state_master (cast `/Game/Blueprints/Player/BC_PlayerState_Master` (`Controller.PlayerState` (`GameplayStatics.GetPlayerController` 0))))
  (return _asbc_player_state_master))

(fn `InitializeResourceMap`
  (returns (ResourcesMap :type "Map of /Game/Blueprints/Enums/E_ResourceTypes Enum to /Game/Blueprints/Structs/S_ResourceStorage Structure"))
  (bind _resourcesdatatable (`self.ResourcesDataTable`))
  (bind _outrownames (`DataTableFunctionLibrary.GetDataTableRowNames` _resourcesdatatable))
  (for _array_element _outrownames
    (bind _returnvalue (`|GetDataTableRow` _resourcesdatatable _array_element)
      (:`then`
        (bind (_resourcetype _name _icon _description _startcount) (break `/Game/Blueprints/Structs/S_ResourcesInfo` _returnvalue))
        (`BlueprintMapLibrary.Map_Add` (`self.ResourcesMap`) _resourcetype (make `/Game/Blueprints/Structs/S_ResourceStorage` _name _icon _startcount)))
      (:`RowNotFound`
        (`KismetSystemLibrary.PrintString` "Error in PlayerState: resource data table row not found"))))
  (return (`self.ResourcesMap`)))

(fn `SpendResource`
  (params (ResourceType :type "/Game/Blueprints/Enums/E_ResourceTypes Enum (by ref)") (Count :type Integer))
  (returns (`Success?` :type Boolean))
  (locals (L_ResourceType :type "/Game/Blueprints/Enums/E_ResourceTypes Enum" :default "NewEnumerator0") (L_ResourceCount :type Integer))
  (bind (_value _returnvalue) (`BlueprintMapLibrary.Map_Find` (`self.ResourcesMap`) (`local.L_ResourceType`)))
  (bind (_displayname _displayicon _count) (break `/Game/Blueprints/Structs/S_ResourceStorage` _value))
  (set `local.L_ResourceType` ResourceType)
  (set `local.L_ResourceCount` Count)
  (if _returnvalue
    (if (>= _count (`local.L_ResourceCount`))
      (bind _structout (setmembers `/Game/Blueprints/Structs/S_ResourceStorage` :`StructRef` _value :`Count` (- _count (`local.L_ResourceCount`))))
      (`BlueprintMapLibrary.Map_Add` (`self.ResourcesMap`) (`local.L_ResourceType`) _structout)
      (`self.OnResourceSpend` (`local.L_ResourceType`) _structout)
      (return true)
      (else
        (return false)))
    (else
      (return false))))