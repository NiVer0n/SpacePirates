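; BP_BaseHUD is a base HUD Blueprint that creates and controls the player's HUD widget.
; InitializeHUDWidget stores the player controller, creates the HUD widget, adds it to the viewport and switches input to Game and UI mode.
; Other functions pass resources to the widget's resources bar and show or hide its galaxy command panel.
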(event `self.ReceiveBeginPlay`)

(fn `InitializeHUDWidget`
  (params (PlayerController :type "/Game/Blueprints/Player/BP_CameraController_Master Object Reference"))
  (bind _output_get (set `self.PlayerController` PlayerController))
  (bind _returnvalue (`|CreateWidget` "/Game/Blueprints/Widgets/WB_PlayerHUD.WB_PlayerHUD_C" _output_get))
  (bind _output_get_2 (set `self.WB_PlayerHUD` _returnvalue))
  (`UserWidget.AddToViewport` _output_get_2 0)
  (`WidgetBlueprintLibrary.SetInputMode_GameAndUIEx` (`self.PlayerController`) null "DoNotLock" false))

(fn `InitializeResourceBar`
  (params (Resources :type "Map of /Game/Blueprints/Enums/E_ResourceTypes Enum to /Game/Blueprints/Structs/S_ResourceStorage Structure"))
  (`/Game/Blueprints/Widgets/WB_Resources_Bar.SetResources` (`/Game/Blueprints/Widgets/WB_PlayerHUD.W_Resources_Bar` (`self.WB_PlayerHUD`)) Resources))

(fn `ShowCommandPanel`
  (params (isVisible :type Boolean))
  (bind _wb_commandpanel_galaxy (`/Game/Blueprints/Widgets/WB_PlayerHUD.WB_CommandPanel_Galaxy` (`self.WB_PlayerHUD`)))
  (if isVisible
    (`Widget.SetVisibility` _wb_commandpanel_galaxy "Visible")
    (else
      (`Widget.SetVisibility` _wb_commandpanel_galaxy "Hidden"))))

(fn `UserConstructionScript`)