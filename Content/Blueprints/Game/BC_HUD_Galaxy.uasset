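; HUD controller Blueprint for the galaxy view that owns and exposes the galaxy HUD widget.
; InitializeHUDWidget stores the player controller, creates WB_HUD_Galaxy, adds it to the viewport and switches input to Game and UI.
; Other functions forward to child widgets, passing resources to the resource bar and toggling command panel visibility.
; Its event graph holds only disabled default events, so setup depends on external calls.
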(fn `InitializeHUDWidget`
  (params (PlayerController :type "/Game/Blueprints/Player/BC_CameraController_Master Object Reference"))
  (bind _output_get (set `self.PlayerController` PlayerController))
  (bind _returnvalue (`|CreateWidget` "/Game/Blueprints/Widgets/WB_HUD_Galaxy.WB_HUD_Galaxy_C" _output_get))
  (bind _output_get_2 (set `self.WB_HUD_Galaxy` _returnvalue))
  (`UserWidget.AddToViewport` _output_get_2 0)
  (`WidgetBlueprintLibrary.SetInputMode_GameAndUIEx` (`self.PlayerController`) null "DoNotLock" false))

(fn `InitializeResourceBar`
  (params (Resources :type "Map of /Game/Blueprints/Enums/E_ResourceTypes Enum to /Game/Blueprints/Structs/S_ResourceStorage Structure"))
  (`/Game/Blueprints/Widgets/WB_Resources_Bar.SetResources` (`/Game/Blueprints/Widgets/WB_HUD_Galaxy.W_Resources_Bar` (`self.WB_HUD_Galaxy`)) Resources))

(fn `ShowCommandPanel`
  (params (IsVisible :type Boolean))
  (bind _wb_commandpanel_galaxy (`/Game/Blueprints/Widgets/WB_HUD_Galaxy.WB_CommandPanel_Galaxy` (`self.WB_HUD_Galaxy`)))
  (if IsVisible
    (`Widget.SetVisibility` _wb_commandpanel_galaxy "Visible")
    (else
      (`Widget.SetVisibility` _wb_commandpanel_galaxy "Hidden"))))

(fn `UserConstructionScript`
  (`parent.UserConstructionScript`))