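; BP_BaseGameState is a game state Blueprint that runs the in-game clock and caches the player's camera controller.
; Each Tick, SetGameTime adds delta time divided by GameSpeed to an hour value wrapped at 24, so higher GameSpeed slows the clock.
; SecondsCounter and DaysCounter derive from that wrapped value, the latter using SecondsInDay.
; BeginPlay stores player controller 0 as a BP_CameraController reference.
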(event `self.ReceiveBeginPlay`
  (`self.GetControllerReference`))

(event `self.ReceiveTick`
  (params (DeltaSeconds :type "Float (single-precision)"))
  (`self.SetGameTime` DeltaSeconds (`self.GameSpeed`)))

(fn `SetGameTime`
  (params (DeltaTime :type "Float (double-precision)") (GameSpeed :type "Float (double-precision)"))
  (locals (GameTimeL :type "Float (double-precision)"))
  (bind _output_get (set `self.GameTime` (`KismetMathLibrary.FMod` (+ (/ DeltaTime GameSpeed) (`self.GameTime`)) 24.0)))
  (bind _returnvalue (* _output_get 3600.0))
  (set `self.SecondsCounter` (`KismetMathLibrary.FFloor` _returnvalue))
  (set `self.DaysCounter` (`.ReturnValue` (`KismetMathLibrary.FMod` _returnvalue (`KismetMathLibrary.Conv_IntToDouble` (`self.SecondsInDay`))))))

(fn `UserConstructionScript`)