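; Galaxy game state that spawns the galaxy playground and manages the countdown and level loading for raids.
; On BeginPlay it creates the galaxy, then builds a contracts builder from its celestial bodies.
; A looping one-second timer broadcasts countdown updates and its end.
; LoadMap opens a tactical map from celestial bodies minus space stations, though the name lookup returns after checking only the first entry.
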(event `self.ReceiveBeginPlay`
  (`parent.ReceiveBeginPlay`)
  (`self.CreateGalaxy`)
  (bind _returnvalue (`|GenericCreateObject` "/Game/Blueprints/GameObjects/BC_ContractsBuilder.BC_ContractsBuilder_C" self self (`/Game/Blueprints/GameObjects/BC_Playground_Galaxy.CelestialBodiesObjects` (`self.GalacticHolder`))))
  (bind _output_get (set `self.ContractsBuilder` _returnvalue))
  (`/Game/Blueprints/GameObjects/BC_ContractsBuilder.Begin Play` _output_get))

(fn `AssignBindings`
  (`parent.AssignBindings`)
  (add `self.OnCountdownStarted` (`|CreateDelegate` :!event `StartCountdown`))
  (add `self.OnCountdownEnded` (`|CreateDelegate` :!event `LoadMap`)))

(fn `CreateGalaxy`
  (bind _returnvalue (`|SpawnActorFromClass` "/Game/Blueprints/GameObjects/BC_Playground_Galaxy.BC_Playground_Galaxy_C" (`KismetMathLibrary.MakeTransform` (0.0 0.0 0.0)) "Undefined" "OverrideRootScale" null 100.0 null))
  (set `self.GalacticHolder` _returnvalue))

(fn `GetRaidObjectMap`
  (returns (TacticalMap :type Name))
  (for _array_element (`self.GetRaidObjectsArray`)
    (if (`KismetTextLibrary.EqualEqual_TextText` (`/Game/Blueprints/GameObjects/BC_CelestialBody_Master.ObjectName` _array_element) (`self.TargetName`))
      (return (`/Game/Blueprints/GameObjects/BC_CelestialBody_Master.TacticalMap` _array_element))
      (else
        (`KismetSystemLibrary.PrintString` (`KismetStringLibrary.Concat_StrStr` "Error: can`t find tactical map for " (`KismetTextLibrary.Conv_TextToString` (`self.TargetName`))))
        (return "None")))))

(fn `GetRaidObjectsArray`
  (returns (TargetObjects :type "Array of /Game/Blueprints/GameObjects/BC_CelestialBody_Master Object Reference"))
  (locals (L_TargetArray :type "Array of /Game/Blueprints/GameObjects/BC_CelestialBody_Master Object Reference"))
  (set `local.L_TargetArray` (`/Game/Blueprints/GameObjects/BC_Playground_Galaxy.CelestialBodiesObjects` (`self.GalacticHolder`)))
  (for _array_element (`/Game/Blueprints/GameObjects/BC_Playground_Galaxy.SpaceStationHolders` (`self.GalacticHolder`))
    (`KismetArrayLibrary.Array_RemoveItem` (`local.L_TargetArray`) _array_element))
  (return (`local.L_TargetArray`)))

(fn `LoadMap`
  (`GameplayStatics.OpenLevel` (`self.GetRaidObjectMap`)))

(fn `StartCountdown`
  (bind _returnvalue (`KismetSystemLibrary.K2_SetTimer` null "UpdateCountdown" 1.0 true))
  (set `self.Coutdown` _returnvalue))

(fn `UpdateCountdown`
  (bind _countdownseconds (`self.CountdownSeconds`))
  (set `self.CountdownSeconds` (- (`self.CountdownSeconds`) 1))
  (`self.OnCountdownUpdated` _countdownseconds)
  (if (== _countdownseconds 0)
    (`KismetSystemLibrary.K2_ClearAndInvalidateTimerHandle` (`self.Coutdown`))
    (`self.OnCountdownEnded`)))

(fn `UserConstructionScript`
  (`parent.UserConstructionScript`))