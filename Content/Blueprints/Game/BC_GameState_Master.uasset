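; Master GameState Blueprint that keeps the game clock, counting seconds and days and broadcasting their changes.
; Tick fires OnSecondsChanged when the fractional part of game time is near zero, an event BeginPlay binds after requesting the camera controller reference.
; UpdateGameDay increments CurrentDay and fires OnDayEnded on SecondsInDay multiples, using a DayUpdated flag against repeated fires.
; SetGameTime_Old retains an older 24-hour wrapping calculation.
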(event `self.ReceiveBeginPlay`
  (`self.GetControllerReference`)
  (add `self.OnSecondsChanged` (`|CreateDelegate` :!event `UpdateGameDay`)))

(event `self.ReceiveTick`
  (params (DeltaSeconds :type "Float (single-precision)"))
  (`self.UpdateGameTime`))

(fn `SetGameTime_Old`
  (params (DeltaTime :type "Float (double-precision)") (GameSpeed :type "Float (double-precision)"))
  (locals (L_GameTime :type "Float (double-precision)" :default 0.01666))
  (bind _output_get (set `local.L_GameTime` (`KismetMathLibrary.FMod` (+ (/ DeltaTime GameSpeed) (`local.L_GameTime`)) 24.0))))

(fn `UpdateGameDay`
  (params (NewSecond :type Integer))
  (if (== (mod NewSecond (`self.SecondsInDay`)) 0)
    (if (not (`self.DayUpdated`))
      (bind _output_get (set `self.CurrentDay` (+ (`self.CurrentDay`) 1)))
      (`self.OnDayEnded` _output_get)
      (set `self.DayUpdated` true))
    (else
      (set `self.DayUpdated` false))))

(fn `UpdateGameTime`
  (bind _returnvalue (`KismetSystemLibrary.GetGameTimeInSeconds`))
  (if (<= (`KismetMathLibrary.Fraction` _returnvalue) 0.04)
    (`self.OnSecondsChanged` (`KismetMathLibrary.FTrunc` _returnvalue))))

(fn `UserConstructionScript`)