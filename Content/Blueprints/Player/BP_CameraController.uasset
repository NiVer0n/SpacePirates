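; Camera controller that drives the BP_CameraSpecator pawn with axis movement, screen-edge panning, rotation and zoom.
; Tick pans the pawn when the mouse nears a viewport edge and CurrentInputState is None, and interpolates spring arm length toward DesiredZoom.
; Holding RotateCamera, if permitted, opens gates so mouse axes yaw the pawn and pitch its camera within limits.
; Zoom inputs step DesiredZoom by a distance-curve amount, clamped to pawn limits.
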(event `self.ReceiveBeginPlay`
  ;[0 0 0] Get Default values
  (`self.GetCameraPawnReference`))

(event `self.ReceiveTick`
  (params (DeltaSeconds :type "Float (single-precision)"))
  ;[0 0 0] Update values in real-time
  (`self.UpdateZoom`)
  (`self.UpdateCamera`))

(event `InputAxis|MoveForward`
  (params (AxisValue :type "Float (single-precision)"))
  ;[0 0 0] Move Camera Input
  (`self.MoveForward/Right` AxisValue (stale `InputAxis|MoveRight` AxisValue) :!label _label))

(event `InputAction|ZoomIn`
  (params (Key :type "Key Structure"))
  ;[0 0 0] Zoom Input
  (:`Pressed`
    (`self.ZoomIn/Out` :!label _label_2)))

(event `InputAxis|MoveRight`
  (params (AxisValue :type "Float (single-precision)"))
  ;[0 0 0] Move Camera Input
  (goto _label :!via `MoveRight`))

(event `InputAction|ZoomOut`
  (params (Key :type "Key Structure"))
  ;[0 0 0] Zoom Input
  (:`Pressed`
    (goto _label_2 :!via `ZoomOut`)))

(event `InputAxisKey|MouseX`
  (params (AxisValue :type "Float (single-precision)"))
  ;[0 0 0] Rotate Camera Events
  (`self.RotateX` AxisValue :!label _label_3))

(event `InputAction|RotateCamera`
  (params (Key :type "Key Structure"))
  ;[0 0 0] Rotate Camera Events
  (:`Pressed`
    (if (`/Game/Blueprints/Player/BP_CameraSpecator.bCanRotateCamera` (`self.CameraPawn`))
      (set `self.CurrentInputState` "NewEnumerator4")
      (goto _label_3 :!via `Open`)))
  (:`Released`
    (set `self.CurrentInputState` "NewEnumerator0")
    (goto _label_3 :!via `Close`)))

(event `InputAxisKey|MouseY`
  (params (AxisValue :type "Float (single-precision)"))
  ;[0 0 0] Rotate Camera Events
  (`self.RotateY` AxisValue :!label _label_4))

(event `InputAction|RotateCamera`
  (params (Key :type "Key Structure"))
  ;[0 0 0] Rotate Camera Events
  (:`Pressed`
    (if (`/Game/Blueprints/Player/BP_CameraSpecator.bCanRotateCamera` (`self.CameraPawn`))
      (set `self.CurrentInputState` "NewEnumerator4")
      (goto _label_4 :!via `Open`)))
  (:`Released`
    (set `self.CurrentInputState` "NewEnumerator0")
    (goto _label_4 :!via `Close`)))

(fn `UserConstructionScript`)