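; Master player state for a galaxy strategy game, holding the player's faction, relationships, resources, build queue and ship hangar.
; Resources initialize from a data table; add and spend functions update the map and fire dispatchers.
; Queuing a unit pays its cost upfront, then a length-adjusted timeline builds units sequentially, announcing each completion.
; A daily event charges maintenance per hangar ship; build and maintenance costs use only their first resource entry.
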(event `self.ReceiveBeginPlay`
  (`self.SetPlayerFaction` "NewEnumerator0") ; By default we play as pyrates,\nbut it can be changed for possible multiplayer
  (`self.SetRelationships`)
  (`self.InitializeResourceMap`))

(event `StartBuildingUnit`
  (params (BuildTime :type "Float (double-precision)") (QueueIndex :type Integer))
  (bind _buildqueue (`self.BuildQueue`))
  ;[0 0 0] Build new unit during build time
  (`TimelineComponent.SetTimelineLength` (`self.ProccessTimeline`) BuildTime)
  (`Timeline|ProccessTimeline` :!via `PlayFromStart`
    (:`Finished`
      (`self.BuildCompleted` (`|GetArrayItem` (`self.BuildQueue`) QueueIndex))
      (`KismetArrayLibrary.Array_Remove` _buildqueue QueueIndex)
      (if (> (`KismetArrayLibrary.Array_Length` _buildqueue) 0)
        (`self.StartBuildingUnit` (`.BuildTime` (defaults `/Game/Blueprints/Player/BC_PlayerState_Master` (`|GetArrayItem` (`self.BuildQueue`)))))))))

(event `OnMaintenanceShips`
  (params (NewDay :type Integer))
  ;[0 0 0] Spend resources for ships maintenance each day`s end
  (bind _keys (`BlueprintMapLibrary.Map_Keys` (`self.UnitsInHangar`)))
  (for _array_element _keys
    (for _ (range 1 (+ (`BlueprintMapLibrary.Map_Find` (`self.UnitsInHangar`) _array_element) 1))
      (bind (_displayname _icon _buildcost _maintenancecost) (defaults `/Game/Blueprints/Player/BC_PlayerState_Master` _array_element))
      (bind _keys_2 (`BlueprintMapLibrary.Map_Keys` _maintenancecost))
      (bind _values (`BlueprintMapLibrary.Map_Values` _maintenancecost))
      (`self.SpendResource` (`|GetArrayItem` _keys_2) (`|GetArrayItem` _values)))))

(fn `AddResource`
  (params (ResourceType :type "/Game/Blueprints/Enums/E_ResourceTypes Enum" :default "NewEnumerator0") (Count :type Integer))
  (returns (`Success?` :type Boolean))
  (bind (_value _returnvalue) (`BlueprintMapLibrary.Map_Find` (`self.ResourcesMap`) ResourceType))
  (if _returnvalue
    (bind _structout (setmembers `/Game/Blueprints/Structs/S_ResourceStorage` :`StructRef` _value :`Count` (+ (`.Count_8_443DEF174797DB10D7CFFD9D13AF4340` (break `/Game/Blueprints/Structs/S_ResourceStorage` _value)) Count)))
    (`BlueprintMapLibrary.Map_Add` (`self.ResourcesMap`) ResourceType _structout)
    (`self.ResourceAdded` ResourceType _structout)
    (return true)
    (else
      (return false))))

(fn `AddToBuildQueue`
  (params (BuildableClass :type "/Game/Blueprints/GameObjects/BC_Unit_Master Class Reference"))
  (locals (L_BuildableClass :type "/Game/Blueprints/GameObjects/BC_Unit_Master Class Reference"))
  (bind (_displayname _icon _buildcost) (defaults `/Game/Blueprints/Player/BC_PlayerState_Master` BuildableClass))
  (bind _l_buildableclass (`local.L_BuildableClass`))
  (set `local.L_BuildableClass` BuildableClass)
  (bind _keys (`BlueprintMapLibrary.Map_Keys` _buildcost))
  (bind _values (`BlueprintMapLibrary.Map_Values` _buildcost))
  (bind _success_ (`self.SpendResource` (`|GetArrayItem` _keys) (`|GetArrayItem` _values)))
  (if _success_
    (if (> (`KismetArrayLibrary.Array_Length` (`self.BuildQueue`)) 0)
      (`KismetArrayLibrary.Array_Add` (`self.BuildQueue`) (`local.L_BuildableClass`))
      (else
        (bind _returnvalue (`KismetArrayLibrary.Array_Add` (`self.BuildQueue`) _l_buildableclass))
        (`self.StartBuildingUnit` (`.BuildTime` (defaults `/Game/Blueprints/Player/BC_PlayerState_Master` _l_buildableclass)) _returnvalue)))))

(fn `AddUnitToHangar`
  (params (Unit :type "/Game/Blueprints/GameObjects/BC_Unit_Master Class Reference"))
  (returns (`Exist?` :type Boolean))
  (locals (L_Unit :type "/Game/Blueprints/GameObjects/BC_Unit_Master Class Reference"))
  (set `local.L_Unit` Unit)
  (if (`BlueprintMapLibrary.Map_Contains` (`self.UnitsInHangar`) (`local.L_Unit`))
    (`BlueprintMapLibrary.Map_Add` (`self.UnitsInHangar`) (`local.L_Unit`) (+ (`BlueprintMapLibrary.Map_Find` (`self.UnitsInHangar`) (`local.L_Unit`)) 1))
    (return true)
    (else
      (`BlueprintMapLibrary.Map_Add` (`self.UnitsInHangar`) (`local.L_Unit`) 1)
      (return false))))

(fn `GetGalaxyGameState`
  (returns (GameState :type "/Game/Blueprints/Game/BC_GameState_Galaxy Object Reference"))
  (bind _asbc_game_state_galaxy (cast `/Game/Blueprints/Game/BC_GameState_Galaxy` (`GameplayStatics.GetGameState`)))
  (return _asbc_game_state_galaxy))

(fn `GetPlayerFaction`
  (returns (PlayerFaction :type "/Game/Blueprints/Enums/E_Faction Enum"))
  (return (`self.PlayerFaction`)))

(fn `GetRelationships`
  (params (Faction :type "/Game/Blueprints/Enums/E_Faction Enum" :default "NewEnumerator0"))
  (returns (Relationships :type "/Game/Blueprints/Enums/E_Relationships Enum"))
  (bind (_value _returnvalue) (`BlueprintMapLibrary.Map_Find` (`self.Relationships`) Faction))
  (if _returnvalue
    (return _value)
    (else
      (return "NewEnumerator2"))))

(fn `InitializeResourceMap`
  (bind _returnvalue (`|GetDataTableRow` (`self.ResourcesDataTable`) "CREDITS")
    (:`then`
      (bind _returnvalue_2 (`|GetDataTableRow` (`self.ResourcesDataTable`) "GAS")
        (:`then`
          (bind _returnvalue_3 (`|GetDataTableRow` (`self.ResourcesDataTable`) "METAL")
            (:`then`
              (bind (_name _icon) (break `/Game/Blueprints/Structs/S_ResourcesInfo` _returnvalue))
              (bind (_name_2 _icon_2) (break `/Game/Blueprints/Structs/S_ResourcesInfo` _returnvalue_2))
              (bind (_name_3 _icon_3) (break `/Game/Blueprints/Structs/S_ResourcesInfo` _returnvalue_3))
              (set `self.ResourcesMap` (`|MakeMap` "NewEnumerator0" (make `/Game/Blueprints/Structs/S_ResourceStorage` _name _icon (`self.CreditsStartValue`)) "NewEnumerator1" (make `/Game/Blueprints/Structs/S_ResourceStorage` _name_2 _icon_2 (`self.GasStartValue`)) "NewEnumerator2" (make `/Game/Blueprints/Structs/S_ResourceStorage` _name_3 _icon_3 (`self.MetalStartValue`)) :!type "/Game/Blueprints/Enums/E_ResourceTypes Enum")))
            (:`RowNotFound`
              (`KismetSystemLibrary.PrintString` "Error in PlayerState: resource data table row not found" :!label _label))))
        (:`RowNotFound`
          (goto _label))))
    (:`RowNotFound`
      (goto _label))))

(fn `SetPlayerFaction`
  (params (PlayerFaction :type "/Game/Blueprints/Enums/E_Faction Enum" :default "NewEnumerator0"))
  (set `self.PlayerFaction` PlayerFaction)
  (`self.OnFactionChanged`))

(fn `SetRelationships`
  (`BlueprintMapLibrary.Map_Clear` (`self.Relationships`))
  ;[0.07227 0.6939 0.1274] Faction 1
  (`BlueprintMapLibrary.Map_Add` (`self.Relationships`) (enumliteral `/Game/Blueprints/Enums/E_Faction` "NewEnumerator0") (select `bool` (`|EnumEquality` (`self.PlayerFaction`) "NewEnumerator0") :`false` (enumliteral `/Game/Blueprints/Enums/E_Relationships` "NewEnumerator2") :`true` (enumliteral `/Game/Blueprints/Enums/E_Relationships` "NewEnumerator1")))
  ;[1 0.2314 0.1882] Faction 2
  (`BlueprintMapLibrary.Map_Add` (`self.Relationships`) (enumliteral `/Game/Blueprints/Enums/E_Faction` "NewEnumerator1") (select `bool` (`|EnumEquality` (`self.PlayerFaction`) "NewEnumerator1") :`false` (enumliteral `/Game/Blueprints/Enums/E_Relationships` "NewEnumerator2") :`true` (enumliteral `/Game/Blueprints/Enums/E_Relationships` "NewEnumerator1")))
  ;[0.5569 0.5569 0.5765] Neutrals
  (`BlueprintMapLibrary.Map_Add` (`self.Relationships`) (enumliteral `/Game/Blueprints/Enums/E_Faction` "NewEnumerator2") (enumliteral `/Game/Blueprints/Enums/E_Relationships` "NewEnumerator2")))

(fn `SpendResource`
  (params (ResourceType :type "/Game/Blueprints/Enums/E_ResourceTypes Enum" :default "NewEnumerator0") (Count :type Integer))
  (returns (`Success?` :type Boolean))
  (bind (_value _returnvalue) (`BlueprintMapLibrary.Map_Find` (`self.ResourcesMap`) ResourceType))
  (bind (_displayname _displayicon _count) (break `/Game/Blueprints/Structs/S_ResourceStorage` _value))
  (if _returnvalue
    (if (>= _count Count)
      (bind _structout (setmembers `/Game/Blueprints/Structs/S_ResourceStorage` :`StructRef` _value :`Count` (- _count Count)))
      (`BlueprintMapLibrary.Map_Add` (`self.ResourcesMap`) ResourceType _structout)
      (`self.ResourceSpent` ResourceType _structout)
      (return true)
      (else
        (return false)))
    (else
      (return false))))

(fn `UserConstructionScript`)