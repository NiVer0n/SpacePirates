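; Master player controller for a top-down, strategy-style camera, driving a BC_CameraSpecator_Master pawn.
; Axis input moves the pawn, Tick edge-scrolls it when no input state is active, and MoveCameraToLocation teleports it for minimap clicks.
; Holding RotateCamera opens gates for mouse yaw on the pawn and clamped pitch on its camera.
; Mouse buttons forward to a constructed BC_InputReceiver; curve-scaled, interpolated zoom helpers are defined but not called here.
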(event `self.ReceiveBeginPlay`
  ;[0 0 0] Get Default values
  (`self.InitializeInputReceiver`))

(event `self.ReceiveTick`
  (params (DeltaSeconds :type "Float (single-precision)"))
  ;[0 0 0] Update values in real-time
  (`self.UpdateCamera`))

(event `InputAxis|MoveForward`
  (params (AxisValue :type "Float (single-precision)"))
  ;[0 0 0] Move Camera Input
  (`self.MoveForward/Right` AxisValue (stale `InputAxis|MoveRight` AxisValue) :!label _label))

(event `InputAxisKey|MouseX`
  (params (AxisValue :type "Float (single-precision)"))
  ;[0 0 0] Rotate Camera Events
  (`self.RotateX` AxisValue :!label _label_2))

(event `InputAction|RotateCamera`
  (params (Key :type "Key Structure"))
  ;[0 0 0] Rotate Camera Events
  (:`Pressed`
    (if (`/Game/Blueprints/Player/BC_CameraSpecator_Master.bCanRotateCamera` (`self.CameraPawn`))
      (set `self.CurrentInputState` "NewEnumerator4")
      (goto _label_2 :!via `Open`)))
  (:`Released`
    (set `self.CurrentInputState` "NewEnumerator0")
    (goto _label_2 :!via `Close`)))

(event `InputAxis|MoveRight`
  (params (AxisValue :type "Float (single-precision)"))
  ;[0 0 0] Move Camera Input
  (goto _label :!via `MoveRight`))

(event `MoveCameraToLocation`
  (params (DestLocation :type "Vector Structure"))
  ;[0 0 0] Move Camera to location (for click on minimap)
  (`self.K2_TeleportTo` (`self.CameraPawn`) DestLocation (`self.K2_GetActorRotation`)))

(event `InputAxisKey|MouseY`
  (params (AxisValue :type "Float (single-precision)"))
  ;[0 0 0] Rotate Camera Events
  (`self.RotateY` AxisValue :!label _label_3))

(event `InputAction|RotateCamera`
  (params (Key :type "Key Structure"))
  ;[0 0 0] Rotate Camera Events
  (:`Pressed`
    (if (`/Game/Blueprints/Player/BC_CameraSpecator_Master.bCanRotateCamera` (`self.CameraPawn`))
      (set `self.CurrentInputState` "NewEnumerator4")
      (goto _label_3 :!via `Open`)))
  (:`Released`
    (set `self.CurrentInputState` "NewEnumerator0")
    (goto _label_3 :!via `Close`)))

(event `Key|LeftMouseButton`
  (params (Key :type "Key Structure"))
  (:`Pressed`
    (bind _inputreceiver (`self.InputReceiver`)
      (:`then`
        (`/Game/Blueprints/GameObjects/BC_InputReceiver.OnLeftMouseButtonDown` _inputreceiver Key))
      (:`else`)))
  (:`Released`
    (bind _inputreceiver_2 (`self.InputReceiver`)
      (:`then`
        (`/Game/Blueprints/GameObjects/BC_InputReceiver.OnLeftMouseButtonUp` _inputreceiver_2 Key))
      (:`else`))))

(event `Key|RightMouseButton`
  (params (Key :type "Key Structure"))
  (:`Pressed`
    (bind _inputreceiver (`self.InputReceiver`)
      (:`then`
        (`/Game/Blueprints/GameObjects/BC_InputReceiver.OnRightMouseButtonDown` _inputreceiver Key))
      (:`else`)))
  (:`Released`
    (bind _inputreceiver_2 (`self.InputReceiver`)
      (:`then`
        (`/Game/Blueprints/GameObjects/BC_InputReceiver.OnRightMouseButtonUp` _inputreceiver_2 Key))
      (:`else`))))

(fn `GetCameraPawnReference`
  (bind _asbc_camera_specator_master (cast `/Game/Blueprints/Player/BC_CameraSpecator_Master` (`self.K2_GetPawn`)))
  (set `self.CameraPawn` _asbc_camera_specator_master))

(fn `GetMousePositionInWorldSpace`
  (returns (Minus :type "Vector Structure") (Plus :type "Vector Structure"))
  (bind (_worldlocation _worlddirection) (`self.DeprojectMousePositionToWorld`))
  (bind _returnvalue (* _worlddirection (/ (.z _worldlocation) (.z _worlddirection))))
  (return (- _worldlocation _returnvalue) (+ _worldlocation _returnvalue)))

(fn `InitializeInputReceiver`
  (bind _returnvalue (`|GenericCreateObject` "/Game/Blueprints/GameObjects/BC_InputReceiver.BC_InputReceiver_C" self self))
  (set `self.InputReceiver` _returnvalue))

(fn `UpdateZoom`
  (bind _camerapawn (`self.CameraPawn`))
  (bind _camerapawn_2 (`self.CameraPawn`))
  ;[0 0 0] Smooth interpolate to new value
  (bind _output_get (set `/Game/Blueprints/Player/BC_CameraSpecator_Master.CurrentZoom` (`KismetMathLibrary.FInterpTo` (`/Game/Blueprints/Player/BC_CameraSpecator_Master.CurrentZoom` _camerapawn) (`/Game/Blueprints/Player/BC_CameraSpecator_Master.DesiredZoom` _camerapawn) (`GameplayStatics.GetWorldDeltaSeconds`) (`/Game/Blueprints/Player/BC_CameraSpecator_Master.ZoomSpeed` _camerapawn)) _camerapawn_2))
  (set `SpringArmComponent.TargetArmLength` _output_get (`/Game/Blueprints/Player/BC_CameraSpecator_Master.SpringArm` _camerapawn_2)))

(fn `UserConstructionScript`)