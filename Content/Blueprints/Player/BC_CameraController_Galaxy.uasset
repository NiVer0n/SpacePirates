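; Galaxy-view player controller that handles celestial object selection and zooming the spectator camera into and out of the selected object.
; On BeginPlay it caches camera pawn, HUD and player state references.
; Zooming in blocks edge scrolling, glides the pawn to the object with camera lag off, and hides its selection marker.
; Timelines ease spring-arm length, DoOnce gates prevent mid-zoom reversal, and the HUD command panel follows zoom for objects with space stations.
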(event `self.ReceiveBeginPlay`
  (`parent.ReceiveBeginPlay`)
  (`self.GetCameraPawnReference`)
  (`self.GetHUDReference`)
  (`/Game/Blueprints/Game/BC_HUD_Master.InitializeHUDWidget` (`self.HUDGalaxy`) self)
  (`self.GetPlayerStateReference`))

(event `self.ReceiveTick`
  (params (DeltaSeconds :type "Float (single-precision)"))
  (`self.UpdateZoom`)
  (`parent.ReceiveTick` DeltaSeconds))

(event `InputAction|ZoomIn`
  (params (Key :type "Key Structure"))
  ;[0 0 0] Zoom Input
  (:`Pressed`
    (`self.ZoomForm/ToObject` :!label _label)))

(event `InputAction|Select`
  (params (Key :type "Key Structure"))
  ;[0 0 0] Select/Deselect Input
  (:`Pressed`
    (if (not (`self.IsZoomed`))
      (`self.SelectObject`))))

(event `InputAction|ZoomOut`
  (params (Key :type "Key Structure"))
  ;[0 0 0] Zoom Input
  (:`Pressed`
    (goto _label :!via `ZoomOut`)))

(fn `GetCameraPawnReference`
  (bind _asbc_camera_specator_galaxy (cast `/Game/Blueprints/Player/BC_CameraSpecator_Galaxy` (`self.K2_GetPawn`)))
  (set `self.CameraPawn` _asbc_camera_specator_galaxy))

(fn `GetHUDReference`
  (bind _asbc_hud_galaxy (cast `/Game/Blueprints/Game/BC_HUD_Galaxy` (`self.GetHUD`)))
  (set `self.HUDGalaxy` _asbc_hud_galaxy))

(fn `GetPlayerStateReference`
  (bind _asbc_player_state_galaxy (cast `/Game/Blueprints/Player/BC_PlayerState_Galaxy` (`self.PlayerState`)))
  (bind _output_get (set `self.Player State` _asbc_player_state_galaxy))
  (set `/Game/Blueprints/Player/BC_PlayerState_Master.PlayerController` self _output_get))

(fn `GetZoomedCameraLocation`
  (returns (ReturnValue :type "Vector Structure"))
  (locals (L_CurrentLocation :type "Vector Structure" :default (0.0 0.0 0.0)) (L_DesiredLocation :type "Vector Structure" :default (0.0 0.0 0.0)))
  (set `local.L_CurrentLocation` (`self.K2_GetActorLocation` (`self.CameraPawn`)))
  (set `local.L_DesiredLocation` (- (`self.K2_GetActorLocation` (`self.SelectedObject`)) (select `bool` (`self.HasSpaceStation`) :`true` (`self.ZoomedCameraOffset`))))
  (return (`KismetMathLibrary.VInterpTo` (`local.L_CurrentLocation`) (`local.L_DesiredLocation`) (`GameplayStatics.GetWorldDeltaSeconds`) (`/Game/Blueprints/Player/BC_CameraSpecator_Master.ZoomSpeed` (`self.CameraPawn`)))))

(fn `HasSpaceStation`
  (returns (HasSpaceSation :type Boolean))
  (bind _asbc_celestial_body_master (cast `/Game/Blueprints/GameObjects/BC_CelestialBody_Master` (`self.SelectedObject`)))
  (`/Engine/EditorBlueprintResources/StandardMacros.IsValid` _asbc_celestial_body_master
    (:`Is Valid`
      (return (`/Game/Blueprints/GameObjects/BC_CelestialBody_Master.HasSpaceStation` _asbc_celestial_body_master)))))

(fn `UserConstructionScript`
  (`parent.UserConstructionScript`))