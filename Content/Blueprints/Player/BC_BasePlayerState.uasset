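; Base player state that tracks the player's credits, gas and metal as a map of resource structs.
; On BeginPlay it caches the camera controller and HUD, waits briefly for the HUD, builds the map from data table rows and start values, and initializes the HUD resource bar.
; AddResource and SpendResource update counts, broadcast change events and return success, with spending refused when funds are insufficient.
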(event `self.ReceiveBeginPlay`
  (`self.GetPlayerControllerReference`)
  (`self.GetHUDReference`)
  (`KismetSystemLibrary.Delay` 0.2) ; Player State initialized earlier than HUD
  (`self.InitializeResourceMap`)
  (`/Game/Blueprints/Game/BP_BaseHUD.InitializeResourcesBar` (`self.HUD`) (`self.ResourcesMap`)))

(fn `AddResource`
  (params (ResourceType :type "/Game/Blueprints/Enums/E_ResourceTypes Enum" :default "NewEnumerator0") (Count :type Integer))
  (returns (`Success?` :type Boolean))
  (bind (_value _returnvalue) (`BlueprintMapLibrary.Map_Find` (`self.ResourcesMap`) ResourceType))
  (if _returnvalue
    (bind _structout (setmembers `/Game/Blueprints/Structs/S_ResourceStorage` :`StructRef` _value :`Count` (+ (`.Count_8_443DEF174797DB10D7CFFD9D13AF4340` (break `/Game/Blueprints/Structs/S_ResourceStorage` _value)) Count)))
    (`BlueprintMapLibrary.Map_Add` (`self.ResourcesMap`) ResourceType _structout)
    (`self.ResourceAdded` ResourceType _structout)
    (return true)
    (else
      (return false))))

(fn `InitializeResourceMap`
  (bind _returnvalue (`|GetDataTableRow` (`self.ResourcesDataTable`) "CREDITS")
    (:`then`
      (bind _returnvalue_2 (`|GetDataTableRow` (`self.ResourcesDataTable`) "GAS")
        (:`then`
          (bind _returnvalue_3 (`|GetDataTableRow` (`self.ResourcesDataTable`) "METAL")
            (:`then`
              (bind (_name _icon) (break `/Game/Blueprints/Structs/S_ResourcesInfo` _returnvalue))
              (bind (_name_2 _icon_2) (break `/Game/Blueprints/Structs/S_ResourcesInfo` _returnvalue_2))
              (bind (_name_3 _icon_3) (break `/Game/Blueprints/Structs/S_ResourcesInfo` _returnvalue_3))
              (set `self.ResourcesMap` (`|MakeMap` "NewEnumerator0" (make `/Game/Blueprints/Structs/S_ResourceStorage` _name _icon (`self.CreditsStartValue`)) "NewEnumerator1" (make `/Game/Blueprints/Structs/S_ResourceStorage` _name_2 _icon_2 (`self.GasStartValue`)) "NewEnumerator2" (make `/Game/Blueprints/Structs/S_ResourceStorage` _name_3 _icon_3 (`self.MetalStartValue`)) :!type "/Game/Blueprints/Enums/E_ResourceTypes Enum")))
            (:`RowNotFound`
              (`KismetSystemLibrary.PrintString` "Error in PlayerState: resource data table row not found" :!label _label))))
        (:`RowNotFound`
          (goto _label))))
    (:`RowNotFound`
      (goto _label))))

(fn `SpendResource`
  (params (ResourceType :type "/Game/Blueprints/Enums/E_ResourceTypes Enum" :default "NewEnumerator0") (Count :type Integer))
  (returns (`Success?` :type Boolean))
  (bind (_value _returnvalue) (`BlueprintMapLibrary.Map_Find` (`self.ResourcesMap`) ResourceType))
  (bind (_displayname _displayicon _count) (break `/Game/Blueprints/Structs/S_ResourceStorage` _value))
  (if _returnvalue
    (if (>= _count Count)
      (bind _structout (setmembers `/Game/Blueprints/Structs/S_ResourceStorage` :`StructRef` _value :`Count` (- _count Count)))
      (`BlueprintMapLibrary.Map_Add` (`self.ResourcesMap`) ResourceType _structout)
      (`self.ResourceSpent` ResourceType _structout)
      (return true)
      (else
        (return false)))
    (else
      (return false))))

(fn `UserConstructionScript`)