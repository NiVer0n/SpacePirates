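; Player camera controller that drives a BP_CameraSpecator_Master pawn with axis movement, screen-edge panning and gated mouse rotation.
; Tick pans only while input state is None; holding RotateCamera opens gates for pawn yaw and clamped camera pitch.
; Zoom helpers step a clamped target via a distance curve and interpolate spring-arm length, but nothing here calls them.
; R, T and Y are test keys that spend player-state resources.
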(event `InputAxis|MoveForward`
  (params (AxisValue :type "Float (single-precision)"))
  ;[0 0 0] Move Camera Input
  (`self.MoveForward/Right` AxisValue (stale `InputAxis|MoveRight` AxisValue) :!label _label))

(event `self.ReceiveBeginPlay`
  ;[0 0 0] Get Default values
  (`self.GetCameraPawnReference`))

(event `self.ReceiveTick`
  (params (DeltaSeconds :type "Float (single-precision)"))
  ;[0 0 0] Update values in real-time
  (`self.UpdateCamera`))

(event `InputAxis|MoveRight`
  (params (AxisValue :type "Float (single-precision)"))
  ;[0 0 0] Move Camera Input
  (goto _label :!via `MoveRight`))

(event `InputAxisKey|MouseX`
  (params (AxisValue :type "Float (single-precision)"))
  ;[0 0 0] Rotate Camera Events
  (`self.RotateX` AxisValue :!label _label_2))

(event `InputAction|RotateCamera`
  (params (Key :type "Key Structure"))
  ;[0 0 0] Rotate Camera Events
  (:`Pressed`
    (if (`/Game/Blueprints/Player/BP_CameraSpecator_Master.bCanRotateCamera` (`self.CameraPawn`))
      (set `self.CurrentInputState` "NewEnumerator4")
      (goto _label_2 :!via `Open`)))
  (:`Released`
    (set `self.CurrentInputState` "NewEnumerator0")
    (goto _label_2 :!via `Close`)))

(event `InputAxisKey|MouseY`
  (params (AxisValue :type "Float (single-precision)"))
  ;[0 0 0] Rotate Camera Events
  (`self.RotateY` AxisValue :!label _label_3))

(event `InputAction|RotateCamera`
  (params (Key :type "Key Structure"))
  ;[0 0 0] Rotate Camera Events
  (:`Pressed`
    (if (`/Game/Blueprints/Player/BP_CameraSpecator_Master.bCanRotateCamera` (`self.CameraPawn`))
      (set `self.CurrentInputState` "NewEnumerator4")
      (goto _label_3 :!via `Open`)))
  (:`Released`
    (set `self.CurrentInputState` "NewEnumerator0")
    (goto _label_3 :!via `Close`)))

(event `Key|R`
  (params (Key :type "Key Structure"))
  ;[0 0 1] For test resources
  (:`Pressed`
    (bind _asbc_base_player_state (cast `/Game/Blueprints/Player/BC_BasePlayerState` (`self.PlayerState`)))
    (`/Game/Blueprints/Player/BC_BasePlayerState.SpendResource` _asbc_base_player_state "NewEnumerator0" 100)))

(event `Key|T`
  (params (Key :type "Key Structure"))
  ;[0 0 1] For test resources
  (:`Pressed`
    (bind _asbc_base_player_state (cast `/Game/Blueprints/Player/BC_BasePlayerState` (`self.PlayerState`)))
    (`/Game/Blueprints/Player/BC_BasePlayerState.SpendResource` _asbc_base_player_state "NewEnumerator1" 100)))

(event `Key|Y`
  (params (Key :type "Key Structure"))
  ;[0 0 1] For test resources
  (:`Pressed`
    (bind _asbc_base_player_state (cast `/Game/Blueprints/Player/BC_BasePlayerState` (`self.PlayerState`)))
    (`/Game/Blueprints/Player/BC_BasePlayerState.SpendResource` _asbc_base_player_state "NewEnumerator2" 100)))

(fn `UpdateZoom`
  (bind _camerapawn (`self.CameraPawn`))
  (bind _camerapawn_2 (`self.CameraPawn`))
  ;[0 0 0] Smooth interpolate to new value
  (bind _output_get (set `/Game/Blueprints/Player/BP_CameraSpecator_Master.CurrentZoom` (`KismetMathLibrary.FInterpTo` (`/Game/Blueprints/Player/BP_CameraSpecator_Master.CurrentZoom` _camerapawn) (`/Game/Blueprints/Player/BP_CameraSpecator_Master.DesiredZoom` _camerapawn) (`GameplayStatics.GetWorldDeltaSeconds`) (`/Game/Blueprints/Player/BP_CameraSpecator_Master.ZoomSpeed` _camerapawn)) _camerapawn_2))
  (set `SpringArmComponent.TargetArmLength` _output_get (`/Game/Blueprints/Player/BP_CameraSpecator_Master.SpringArm` _camerapawn_2)))

(fn `UserConstructionScript`)