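; Player controller for the tactical camera that routes mouse input and zooms the spectator pawn.
; On BeginPlay it caches the camera pawn, HUD and player state, initializing the HUD and registering itself on the player state.
; Mouse buttons forward to an InputReceiver, while select press, timed hold and release also notify the HUD.
; A zoom macro lerps the pawn relative to the mouse's world position, clamping vector size and suspending camera lag during each move.
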(event `self.ReceiveBeginPlay`
  (`parent.ReceiveBeginPlay`)
  (`self.GetCameraPawnReference`)
  (`self.GetHUDReference`)
  (`/Game/Blueprints/Game/BC_HUD_Master.InitializeHUDWidget` (`self.HUDTactical`) self)
  (`self.GetPlayerStateReference`))

(event `self.ReceiveTick`
  (params (DeltaSeconds :type "Float (single-precision)"))
  (`parent.ReceiveTick` DeltaSeconds)
  (`self.UpdateHoldInput`))

(event `InputAction|Select`
  (params (Key :type "Key Structure"))
  (:`Pressed`
    (bind _inputreceiver (`self.InputReceiver`)
      (:`then`
        (`/Game/Blueprints/GameObjects/BC_InputReceiver.OnLeftMouseButtonDown` _inputreceiver Key)
        (message `/Game/Blueprints/Interfaces/BI_Input.OnInputStart` (`self.HUDTactical`))
        (set `self.InputHoldingTime` 0.0)
        (set `self.IsHoldingInput` true))
      (:`else`)))
  (:`Released`
    (bind _inputreceiver_2 (`self.InputReceiver`)
      (:`then`
        (`/Game/Blueprints/GameObjects/BC_InputReceiver.OnLeftMouseButtonUp` _inputreceiver_2 Key)
        (message `/Game/Blueprints/Interfaces/BI_Input.OnInputRelease` (`self.HUDTactical`) (`self.InputHoldingTime`))
        (set `self.IsHoldingInput` false))
      (:`else`))))

(event `Key|RightMouseButton`
  (params (Key :type "Key Structure"))
  (:`Pressed`
    (bind _inputreceiver (`self.InputReceiver`)
      (:`then`
        (`/Game/Blueprints/GameObjects/BC_InputReceiver.OnRightMouseButtonDown` _inputreceiver Key))
      (:`else`)))
  (:`Released`
    (bind _inputreceiver_2 (`self.InputReceiver`)
      (:`then`
        (`/Game/Blueprints/GameObjects/BC_InputReceiver.OnRightMouseButtonUp` _inputreceiver_2 Key))
      (:`else`))))

(event `InputAction|ZoomIn`
  (params (Key :type "Key Structure"))
  (:`Pressed`
    (`self.ZoomCamera` :!label _label)))

(event `InputAction|ZoomOut`
  (params (Key :type "Key Structure"))
  (:`Pressed`
    (goto _label :!via `ZoomOut`)))

(fn `GetCameraPawnReference`
  (bind _asbc_camera_specator_tactical (cast `/Game/Blueprints/Player/BC_CameraSpecator_Tactical` (`self.K2_GetPawn`)))
  (set `self.CameraPawn` _asbc_camera_specator_tactical))

(fn `GetHUDReference`
  (bind _asbc_hud_tactical (cast `/Game/Blueprints/Game/BC_HUD_Tactical` (`self.GetHUD`)))
  (set `self.HUDTactical` _asbc_hud_tactical))

(fn `GetPlayerStateReference`
  (bind _asbc_player_state_tactical (cast `/Game/Blueprints/Player/BC_PlayerState_Tactical` (`self.PlayerState`)))
  (bind _output_get (set `self.Player State` _asbc_player_state_tactical))
  (set `/Game/Blueprints/Player/BC_PlayerState_Master.PlayerController` self _output_get))

(fn `UpdateHoldInput`
  (if (`self.IsHoldingInput`)
    (set `self.InputHoldingTime` (+ (`GameplayStatics.GetWorldDeltaSeconds`) (`self.InputHoldingTime`)))
    (message `/Game/Blueprints/Interfaces/BI_Input.OnInputHold` (`self.HUDTactical`))))

(fn `UserConstructionScript`
  (`parent.UserConstructionScript`))