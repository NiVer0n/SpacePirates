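; Galaxy-view camera controller that handles zoom and selection of celestial bodies.
; Zoom input lerps the camera pawn toward or away from a deprojected cursor position, clamping vector size to stay inside the skybox and toggling spring-arm lag around each move.
; Select traces under the cursor, toggles the body's name and highlight, and fires selection events.
; An older timeline-driven zoom-to-object macro remains but is never run.
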(event `self.ReceiveTick`
  (params (DeltaSeconds :type "Float (single-precision)"))
  (`self.UpdateZoom`)
  (`parent.ReceiveTick` DeltaSeconds))

(event `InputAction|ZoomIn`
  (params (Key :type "Key Structure"))
  ;[0 0 0] Zoom Input
  (:`Pressed`
    (`self.ZoomIn/Out` :!label _label)))

(event `InputAction|Select`
  (params (Key :type "Key Structure"))
  ;[0 0 0] Select/Deselect Input
  (:`Pressed`
    (`self.SelectObject`)))

(event `InputAction|ZoomOut`
  (params (Key :type "Key Structure"))
  ;[0 0 0] Zoom Input
  (:`Pressed`
    (goto _label :!via `ZoomOut`)))

(fn `UserConstructionScript`
  (`parent.UserConstructionScript`))