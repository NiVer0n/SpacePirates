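; Player state for the tactical mode that fills the HUD resource bar with saved resources when play begins.
; After the parent BeginPlay, it passes the resource map from the save to the tactical HUD's InitializeResourceBar.
; A helper, GetHUDTactical, finds that HUD by casting the player controller to BC_CameraController_Tactical.
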(event `self.ReceiveBeginPlay`
  (`parent.ReceiveBeginPlay`)
  (`/Game/Blueprints/Game/BC_HUD_Galaxy.InitializeResourceBar` (`self.GetHUDTactical`) (`self.GetResourceMapFromSave`)))

(fn `GetHUDTactical`
  (returns (HUD :type "/Game/Blueprints/Game/BC_HUD_Tactical Object Reference"))
  (return (`/Game/Blueprints/Player/BC_CameraController_Tactical.HUDTactical` (cast `/Game/Blueprints/Player/BC_CameraController_Tactical` (`self.PlayerController`) :!pure true))))

(fn `UserConstructionScript`
  (`parent.UserConstructionScript`))