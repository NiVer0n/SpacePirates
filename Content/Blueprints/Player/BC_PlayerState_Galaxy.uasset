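; Player state for the galaxy part of the game that holds the player's resources map and shows it on the galaxy HUD.
; On BeginPlay it runs the parent logic, then initializes the HUD resource bar from that map.
; The HUD is reached by casting the player controller to the galaxy camera controller.
; AssignBindings subscribes an event to the galaxy game state's day-ended dispatcher.
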(event `self.ReceiveBeginPlay`
  (`parent.ReceiveBeginPlay`)
  (`/Game/Blueprints/Game/BC_HUD_Galaxy.InitializeResourceBar` (`self.GetHUDGalaxy`) (`self.ResourcesMap`)))

(fn `AssignBindings`
  (add `/Game/Blueprints/Game/BC_GameState_Master.OnDayEnded` (`self.GetGalaxyGameState`) (`|CreateDelegate` :!event `OnMaintenanceShips`)))

(fn `GetHUDGalaxy`
  (returns (HUD :type "/Game/Blueprints/Game/BC_HUD_Galaxy Object Reference"))
  (return (`/Game/Blueprints/Player/BC_CameraController_Galaxy.HUDGalaxy` (cast `/Game/Blueprints/Player/BC_CameraController_Galaxy` (`self.PlayerController`) :!pure true))))

(fn `UserConstructionScript`
  (`parent.UserConstructionScript`))