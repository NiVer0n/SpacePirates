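; Ghost preview actor for unit spawn placement, showing the unit's mesh with collision disabled.
; On BeginPlay it creates a dynamic wireframe material in the good-position color and adds it to the UnitMesh asset, rather than overriding the component's materials.
; SetPositionMaterial switches GridColor between good and bad colors, but the position check is a stub returning true.
; The pass applying the material to child submeshes is disconnected.
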(event `self.ReceiveBeginPlay`
  (`StaticMeshComponent.SetStaticMesh` (`self.Mesh`) (`self.UnitMesh`))
  (`self.SetSpawnMaterial`)
  (`self.SetActorEnableCollision` false))

(fn `IsGoodPositionForSpawn`
  (returns (GoodPosition :type Boolean))
  (return true))

(fn `SetPositionMaterial`
  (if (`self.IsGoodPositionForSpawn`)
    (`MaterialInstanceDynamic.SetVectorParameterValue` (`self.WireframeMaterial`) "GridColor" (`self.GoodPositionGhostColor`))
    (else
      (`MaterialInstanceDynamic.SetVectorParameterValue` (`self.WireframeMaterial`) "GridColor" (`self.BadPositionGhostColor`)))))

(fn `SetSpawnMaterial`
  (locals (L_SubmeshStatic :type "StaticMeshComponent Object Reference") (L_SubmeshSkeletal :type "SkeletalMeshComponent Object Reference"))
  (bind _returnvalue (`KismetMaterialLibrary.CreateDynamicMaterialInstance` "/Game/Materials/MM_Wireframe.MM_Wireframe"))
  (`MaterialInstanceDynamic.SetVectorParameterValue` _returnvalue "GridColor" (`self.GoodPositionGhostColor`))
  (set `self.WireframeMaterial` _returnvalue)
  (`StaticMesh.AddMaterial` (`self.UnitMesh`) (`self.WireframeMaterial`)))

(fn `UserConstructionScript`)