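; Blueprint component that generates raid contracts for the game, presumably refreshed through its binding to the GameState's day-ended event.
; UpdateContracts broadcasts an update, then creates a random batch of contracts sized against the remaining MaxContracts capacity.
; Each contract broadcasts a random raid target, duration and bounty type, with a fixed defense level.
; Required fuel is round-trip straight-line distance from the first space station, scaled by FuelCountForPoint.
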(event Custom|Begin%20Play
  (EventDispatchers|BindEventtoOnDayEnded (Variables|References|GetGameState) (EventDispatchers|CreateEvent :!event UpdateContracts)))

(fn CreateContract
  (bind _output_get (LocalVariables|SetL_Target (CallFunction|GetSuitableTarget)))
  (Default|CallOnContractCreated (Variables|/Game/Blueprints/GameObjects/BC_CelestialBody_Master.BC_CelestialBody_Master_C|GetObjectName _output_get) (Math|Random|RandomIntegerinRange (Variables|Gameplay|GetMinContractDuration) (Variables|Gameplay|GetMaxContractDuration)) (CallFunction|GetRequiredFueltoTarget (LocalVariables|GetL_Target)) (Utilities|Select :Index (Math|Random|RandomIntegerinRange 0 2) :Option%200 "NewEnumerator0" :Option%201 "NewEnumerator1" :Option%202 "NewEnumerator2") "NewEnumerator0")
  (Variables|Gameplay|SetCurrentContracts (+ (Variables|Gameplay|GetCurrentContracts) 1)))

(fn GetSuitableTarget
  (LocalVariables|SetL_TargetArray (Default|GetRaidObjectsArray (Variables|References|GetGameState)))
  (return (Utilities|Array|Get(acopy) (LocalVariables|GetL_TargetArray) (Math|Random|RandomIntegerinRange 0 (- (Utilities|Array|Length (LocalVariables|GetL_TargetArray)) 1)))))

(fn GetSuitableContractsCount
  (bind _currentcontracts (Variables|Gameplay|GetCurrentContracts))
  (bind _maxcontracts (Variables|Gameplay|GetMaxContracts))
  (bind _returnvalue (- _maxcontracts _currentcontracts))
  (bind _returnvalue_2 (Math|Random|RandomIntegerinRange 3 _returnvalue))
  (if (<= (+ _returnvalue_2 (Variables|Gameplay|GetCurrentContracts)) (Variables|Gameplay|GetMaxContracts))
    (return _returnvalue_2)
    (else
      (return -1))))

(fn UpdateContracts
  (params (NewDay :type Integer))
  (Default|CallOnContractUpdated)
  (for _index (range 0 (CallFunction|GetSuitableContractsCount))
    (CallFunction|CreateContract)))

(fn CalculateDistance
  (params (From :type BC%20Celestial%20Body%20Master%20Object%20Reference) (To :type BC%20Celestial%20Body%20Master%20Object%20Reference))
  (bind _returnvalue (Transformation|GetActorLocation To))
  (bind _returnvalue_2 (Transformation|GetActorLocation From))
  (bind (_x _y _z) (Math|Vector|BreakVector _returnvalue))
  (bind (_x_2 _y_2 _z_2) (Math|Vector|BreakVector _returnvalue_2))
  (return (|(round((sqrt((((power((x2-x1),2))+(power((y2-y1),2)))+(power((z2-z1),2))))))) _x _x_2 _y _y_2 _z _z_2)))

(fn GetRequiredFueltoTarget
  (params (To :type BC%20Celestial%20Body%20Master%20Object%20Reference))
  (return (* (Math|Float|Round (* (CallFunction|CalculateDistance (Utilities|Array|Get(acopy) (Variables|/Game/Blueprints/GameObjects/BC_Playground_Galaxy.BC_Playground_Galaxy_C|GetSpaceStationHolders (Variables|/Game/Blueprints/Game/BC_GameState_Galaxy.BC_GameState_Galaxy_C|GetGalacticHolder (Variables|References|GetGameState)))) To) (Variables|Gameplay|GetFuelCountForPoint))) 2)))