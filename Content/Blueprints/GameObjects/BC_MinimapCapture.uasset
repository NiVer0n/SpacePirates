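; Minimap capture actor that renders an area of the level through a SceneCaptureComponent2D.
; The construction script uses MinimapSize to set both the capture's ortho width and a thin, square Box matching that footprint.
; The CaptureMap event triggers a single CaptureScene call; BeginPlay does nothing, so this graph captures only when that event is called.
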(event `self.ReceiveBeginPlay`)

(event `CaptureMap`
  (`SceneCaptureComponent2D.CaptureScene` (`self.SceneCaptureComponent2D`)))

(fn `UserConstructionScript`
  (bind _returnvalue (/ (`self.MinimapSize`) 2.0))
  (`BoxComponent.SetBoxExtent` (`self.Box`) (`KismetMathLibrary.MakeVector` 2.0 _returnvalue _returnvalue) true)
  (set `SceneCaptureComponent2D.OrthoWidth` (`self.MinimapSize`) (`self.SceneCaptureComponent2D`)))