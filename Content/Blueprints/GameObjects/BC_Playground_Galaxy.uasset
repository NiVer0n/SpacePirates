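; BC_Playground_Galaxy is the galaxy playground that builds the galactic map and places a parent space station on BeginPlay.
; Each CelestialBodiesDataTable row spawns a celestial body with its position, scale, appearance, tactical map and station settings, making the layout data-driven.
; Bodies flagged CanSpawnParentStation become candidate holders.
; One random candidate then spawns its space station and is recorded in SpaceStationHolders.
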(event `self.ReceiveBeginPlay`
  (`parent.ReceiveBeginPlay`)
  (`self.CreateGalacticMap`)
  (`self.SpawnParentStation`))

(fn `CreateGalacticMap`
  (bind _celestialbodiesdatatable (`self.CelestialBodiesDataTable`))
  (bind _outrownames (`DataTableFunctionLibrary.GetDataTableRowNames` _celestialbodiesdatatable))
  (for _array_element _outrownames
    (bind _returnvalue (`|GetDataTableRow` _celestialbodiesdatatable _array_element)
      (:`then`
        (bind (_objectname _objectclass _galacticposition _objectscale _objectmaterial _tacticalmap _canspawnparentstation _spacesationclass _spacestationoffset _spacestationscale) (break `/Game/Blueprints/Structs/S_CelestialBodyInfo` _returnvalue))
        (bind _returnvalue_2 (`|SpawnActorFromClass` _objectclass (`KismetMathLibrary.MakeTransform` _galacticposition (struct) (`KismetMathLibrary.Conv_DoubleToVector` _objectscale)) "AdjustIfPossibleButDontSpawnIfColliding" "OverrideRootScale" null _objectname _objectmaterial _tacticalmap _spacesationclass _spacestationoffset _spacestationscale null))
        (`KismetArrayLibrary.Array_Add` (`self.CelestialBodiesObjects`) _returnvalue_2)
        (if _canspawnparentstation
          (`KismetArrayLibrary.Array_Add` (`self.PossibleSpaceStationHolders`) _returnvalue_2))))))

(fn `SpawnParentStation`
  (locals (L_StationHolder :type "/Game/Blueprints/GameObjects/BC_CelestialBody_Master Object Reference"))
  (bind _possiblespacestationholders (`self.PossibleSpaceStationHolders`))
  (bind _output_get (set `local.L_StationHolder` (`|GetArrayItem` _possiblespacestationholders (`KismetMathLibrary.RandomIntegerInRange` 0 (- (`KismetArrayLibrary.Array_Length` _possiblespacestationholders) 1)))))
  (`/Game/Blueprints/GameObjects/BC_CelestialBody_Master.SpawnSpaceStation` _output_get)
  (`KismetArrayLibrary.Array_Add` (`self.SpaceStationHolders`) (`local.L_StationHolder`)))

(fn `UserConstructionScript`
  (`parent.UserConstructionScript`))