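; Galactic map master actor that builds the galaxy from celestial body data at BeginPlay.
; Each data entry spawns an actor at its galactic position and scale, passing in name, material, tactical map and space station settings.
; Bodies flagged as able to host the parent station are collected, and one chosen at random spawns its space station.
; The construction script scales the galaxy bounds component in X and Y by the map size.
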(event `self.ReceiveBeginPlay`
  (`self.CreateGalacticMap`)
  (`self.SpawnParentStation`))

(fn `CreateGalacticMap`
  (for _array_element (`self.CelestialBodiesData`)
    (bind (_objectname _objecttype _galacticposition _objectscale _objectmaterial _tacticalmap _canspawnparentstation _spacesationclass _spacestationoffset _spacestationscale) (break `/Game/Blueprints/Structs/S_CelestialBodyInfo` _array_element))
    (bind _returnvalue (`|SpawnActorFromClass` _objecttype (`KismetMathLibrary.MakeTransform` _galacticposition (struct) (`KismetMathLibrary.Conv_DoubleToVector` _objectscale)) "AdjustIfPossibleButDontSpawnIfColliding" "OverrideRootScale" null _objectname _objectmaterial _tacticalmap _spacesationclass _spacestationoffset _spacestationscale null))
    (if _canspawnparentstation
      (`KismetArrayLibrary.Array_Add` (`self.CelestialBodiesActorArray`) _returnvalue))))

(fn `SpawnParentStation`
  (bind _celestialbodiesactorarray (`self.CelestialBodiesActorArray`))
  (`/Game/Blueprints/GameObjects/BC_CelestialBody_Master.SpawnSpaceStation` (`|GetArrayItem` _celestialbodiesactorarray (`KismetMathLibrary.RandomIntegerInRange` 0 (- (`KismetArrayLibrary.Array_Length` _celestialbodiesactorarray) 1)))))

(fn `UserConstructionScript`
  (bind _mapsize (`self.MapSize`))
  (`SceneComponent.SetWorldScale3D` (`self.GalaxyBounds`) (`KismetMathLibrary.MakeVector` _mapsize _mapsize)))