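; Actor component that shows its owner on the player HUD minimap, registering on begin play and unregistering on end play.
; After a short delay for player state and HUD spawning, it reaches the minimap widget through the camera controller's HUD.
; It normalizes the owner's XY location by the galactic master actor's bounds extent, offset by 0.5.
; It also supplies the owner's controlling faction and a relationship-based icon.
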(event `self.ReceiveBeginPlay`
  (`self.InitializeComponent`))

(event `self.ReceiveEndPlay`
  (params (EndPlayReason :type "EEndPlayReason Enum" :default "Destroyed"))
  (bind _w_minimap (`self.W_Minimap`)
    (:`then`
      (`/Game/Blueprints/Widgets/WB_Minimap.RemoveFromObservables` _w_minimap self))
    (:`else`)))

(event `InitializeComponent`
  (bind _outactors (`GameplayStatics.GetAllActorsOfClass` "/Game/Blueprints/GameObjects/BC_Galactic_Master.BC_Galactic_Master_C"))
  (set `self.LevelSize` (`KismetMathLibrary.Conv_VectorToVector2D` (`.BoxExtent` (`Actor.GetActorBounds` (`|GetArrayItem` _outactors) false))))
  (`KismetSystemLibrary.Delay` 0.1) ; Need for spawn player state and player HUD first
  (bind _asbp_camera_controller_master (cast `/Game/Blueprints/Player/BP_CameraController_Master` (`GameplayStatics.GetPlayerController` 0)))
  (bind _output_get (set `self.W_Minimap` (`/Game/Blueprints/Widgets/WB_PlayerHUD.WB_Minimap` (`/Game/Blueprints/Game/BP_BaseHUD.WB_PlayerHUD` (`/Game/Blueprints/Player/BP_CameraController_Master.HUD` _asbp_camera_controller_master)))))
  (`/Game/Blueprints/Widgets/WB_Minimap.AddObjectToMinimap` _output_get self))

(fn `GetActorFaction`
  (returns (Faction :type "/Game/Blueprints/Enums/E_Faction Enum"))
  (bind _controlledfaction (`/Game/Blueprints/Interfaces/BI_ControlledFaction.GetControlledFaction` (cast `/Game/Blueprints/Interfaces/BI_ControlledFaction` (`self.GetOwner`) :!pure true)))
  (return _controlledfaction))

(fn `GetIcon`
  (params (Relationships :type "/Game/Blueprints/Enums/E_Relationships Enum" :default "NewEnumerator0"))
  (returns (Value :type "Texture2D Object Reference"))
  (return (`BlueprintMapLibrary.Map_Find` (`self.MinimapIcons`) Relationships)))

(fn `GetNormalizedLocation`
  (returns (MapLocation :type "Vector2D Structure"))
  (bind (_x _y) (`KismetMathLibrary.BreakVector2D` (`self.LevelSize`)))
  (return (+ (`KismetMathLibrary.MakeVector2D` (/ (.x (`Actor.K2_GetActorLocation` (`self.GetOwner`))) _x) (/ (.y (`Actor.K2_GetActorLocation` (`self.GetOwner`))) _y)) 0.5)))