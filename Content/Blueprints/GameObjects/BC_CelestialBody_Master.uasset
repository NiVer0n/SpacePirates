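; BC_CelestialBody_Master is a celestial body actor, named as a master class, with a mesh, a selection indicator and a name widget.
; Construction applies the configured material to the mesh, and BeginPlay copies the object's name into its WB_CelestialBodyName widget.
; Cursor hover shows and hides the name unless the body is selected.
; Separate functions expose visibility control for the selection indicator and name.
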(event `self.ReceiveBeginPlay`
  (`self.SetCelestialBodyName`))

(event `self.ReceiveActorBeginCursorOver`
  (if (not (`self.isSelected`))
    (`self.SetNameVisibility` true)))

(event `self.ReceiveActorEndCursorOver`
  (if (not (`self.isSelected`))
    (`self.SetNameVisibility` false)))

(fn `SetNameVisibility`
  (params (Visibility :type Boolean))
  (`SceneComponent.SetVisibility` (`self.Name Widget`) Visibility false))

(fn `SetSelectionVisibility`
  (params (Visibility :type Boolean))
  (`SceneComponent.SetVisibility` (`self.ObjectSelection`) Visibility false))

(fn `UserConstructionScript`
  (`PrimitiveComponent.SetMaterial` (`self.ObjectMesh`) 0 (`self.ObjectMaterial`)))